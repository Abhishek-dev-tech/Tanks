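; Tanks game mode that switches the on-screen UI between menu, playing and game-over states.
; StartGame adds the menu widget to the viewport and shows the mouse cursor for the first player controller.
; StartPlaying and GameOver each clear all widgets, then add their own screen.
; The graph holds only this UI switching, with no calls to these events and no gameplay rules.
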(event `self.StartGame`
  (bind _returnvalue (`|CreateWidget` "/Game/Blueprints/Widget/WBP_Menu.WBP_Menu_C"))
  (`UserWidget.AddToViewport` _returnvalue 0)
  (set `PlayerController.bShowMouseCursor` true (`GameplayStatics.GetPlayerController` 0)))

(event `self.StartPlaying`
  (`WidgetLayoutLibrary.RemoveAllWidgets`)
  (bind _returnvalue (`|CreateWidget` "/Game/Blueprints/Widget/WBP_Playing.WBP_Playing_C"))
  (`UserWidget.AddToViewport` _returnvalue 0))

(event `self.GameOver`
  (`WidgetLayoutLibrary.RemoveAllWidgets`)
  (bind _returnvalue (`|CreateWidget` "/Game/Blueprints/Widget/WBP_GameOver.WBP_GameOver_C"))
  (`UserWidget.AddToViewport` _returnvalue 0))

(fn `UserConstructionScript`)